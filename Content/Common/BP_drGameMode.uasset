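; Game mode that, on BeginPlay, creates the UI widgets, shows Login and converts saved-directory text files into an ADataSave slot.
; ChangeData parses numbered files into object transform and ID records using nested string splits, stopping at the first failed load.
; ChangeLightData parses PA and SA files into type 1 and 2 lights, then saves both arrays, overwriting the same slot "14403".
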(event EventBeginPlay
  (bind _returnvalue (UserInterface|CreateWidget "/Game/Business/UMG/Login.Login_C"))
  (bind _output_get (Variables|Default|SetLoginUI _returnvalue))
  (UserInterface|Viewport|AddtoViewport _output_get 0)
  (bind _returnvalue_2 (UserInterface|CreateWidget "/Game/Business/UMG/Main.Main_C"))
  (Variables|Default|SetMainUI _returnvalue_2)
  (bind _returnvalue_3 (UserInterface|CreateWidget "/Game/Business/UMG/Loading.Loading_C"))
  (Variables|Default|SetLoadingUI _returnvalue_3)
  (bind _returnvalue_4 (UserInterface|CreateWidget "/Game/Business/UMG/3DMain.3DMain_C"))
  (Variables|Default|Set3DMainUI _returnvalue_4)
  (CallFunction|ChangeData)
  (CallFunction|ChangeLightData))

(event EventTick
  (params (DeltaSeconds :type Float%20%28single-precision%29)))

(fn ConstructionScript)

(fn ChangeData
  (bind (_contents _returnvalue) (Class|BuildingSystem|LoadStringfromFile (Utilities|String|Append (Class|KismetSystemLibrary|GetProjectSavedDirectory) (Utilities|String|ToString(Integer) (Variables|Default|GetNewVar_0)) ".txt") :!label _label))
  (if _returnvalue
    (Utilities|Array|Add (Variables|Default|GetNewVar_1) (Utilities|Struct|MakeAData (Math|Conversions|ToInteger(Byte) (.LeftS (Utilities|String|Split _contents "+"))) (Math|Conversions|ToInteger(Byte) (.LeftS (Utilities|String|Split (.RightS (Utilities|String|Split _contents "+")) "+"))) -1 (Math|Vector|MakeVector (Math|Conversions|ToFloat(Integer) (.RightS (Utilities|String|Split (.LeftS (Utilities|String|Split (.LeftS (Utilities|String|Split (.RightS (Utilities|String|Split (.RightS (Utilities|String|Split _contents "+")) "+")) "+")) "Y")) "="))) (Math|Conversions|ToFloat(Integer) (.RightS (Utilities|String|Split (.LeftS (Utilities|String|Split (.LeftS (Utilities|String|Split (.RightS (Utilities|String|Split (.RightS (Utilities|String|Split _contents "+")) "+")) "+")) "Z")) "=" "IgnoreCase" "FromEnd"))) (Math|Conversions|ToFloat(Integer) (.RightS (Utilities|String|Split (.LeftS (Utilities|String|Split (.RightS (Utilities|String|Split (.RightS (Utilities|String|Split _contents "+")) "+")) "+")) "=" "IgnoreCase" "FromEnd")))) (Math|Rotator|MakeRotator (Math|Conversions|ToFloat(Integer) (.RightS (Utilities|String|Split (.LeftS (Utilities|String|Split (.LeftS (Utilities|String|Split (.RightS (Utilities|String|Split (.RightS (Utilities|String|Split (.RightS (Utilities|String|Split _contents "+")) "+")) "+")) "+")) "Y")) "="))) (Math|Conversions|ToFloat(Integer) (.RightS (Utilities|String|Split (.LeftS (Utilities|String|Split (.LeftS (Utilities|String|Split (.RightS (Utilities|String|Split (.RightS (Utilities|String|Split (.RightS (Utilities|String|Split _contents "+")) "+")) "+")) "+")) "R")) "=" "IgnoreCase" "FromEnd"))) (Math|Conversions|ToFloat(Integer) (.RightS (Utilities|String|Split (.LeftS (Utilities|String|Split (.RightS (Utilities|String|Split (.RightS (Utilities|String|Split (.RightS (Utilities|String|Split _contents "+")) "+")) "+")) "+")) "=" "IgnoreCase" "FromEnd")))) (Math|Vector|MakeVector (Math|Conversions|ToFloat(Integer) (.RightS (Utilities|String|Split (.LeftS (Utilities|String|Split (.LeftS (Utilities|String|Split (.RightS (Utilities|String|Split (.RightS (Utilities|String|Split (.RightS (Utilities|String|Split (.RightS (Utilities|String|Split _contents "+")) "+")) "+")) "+")) "+")) "Y")) "="))) (Math|Conversions|ToFloat(Integer) (.RightS (Utilities|String|Split (.LeftS (Utilities|String|Split (.LeftS (Utilities|String|Split (.RightS (Utilities|String|Split (.RightS (Utilities|String|Split (.RightS (Utilities|String|Split (.RightS (Utilities|String|Split _contents "+")) "+")) "+")) "+")) "+")) "Z")) "=" "IgnoreCase" "FromEnd"))) (Math|Conversions|ToFloat(Integer) (.RightS (Utilities|String|Split (.LeftS (Utilities|String|Split (.RightS (Utilities|String|Split (.RightS (Utilities|String|Split (.RightS (Utilities|String|Split (.RightS (Utilities|String|Split _contents "+")) "+")) "+")) "+")) "+")) "=" "IgnoreCase" "FromEnd")))) (.RightS (Utilities|String|Split (.RightS (Utilities|String|Split (.RightS (Utilities|String|Split (.RightS (Utilities|String|Split (.RightS (Utilities|String|Split _contents "+")) "+")) "+")) "+")) "+"))))
    (bind _result (Math|Integer|IncrementInt (Variables|Default|GetNewVar_0))
      (:%20%20
        (if (> _result 287)
          (bind _returnvalue_2 (SaveGame|CreateSaveGameObject "/Game/Common/ADataSave.ADataSave_C"))
          (Variables|/Game/Common/ADataSave.ADataSave_C|SetAData _returnvalue_2 (Variables|Default|GetNewVar_1))
          (bind _returnvalue_3 (SaveGame|SaveGametoSlot _returnvalue_2 "14403"))
          (if _returnvalue_3
            (Development|PrintString "Hello")
            (else
              (Development|PrintString "Hello")))
          (else
            (goto _label)))))))

(fn ChangeLightData
  (for _array_element (Variables|Default|GetNewVar_2)
    (bind (_contents _returnvalue) (Class|BuildingSystem|LoadStringfromFile (Utilities|String|Append (Class|KismetSystemLibrary|GetProjectSavedDirectory) "PA" (Utilities|String|ToString(Integer) _array_element))))
    (if _returnvalue
      (Utilities|Array|Add (Variables|Default|GetNewVar_3) (Utilities|Struct|MakeLightData (Math|Conversions|ToInteger(Byte) (.LeftS (Utilities|String|Split _contents "+"))) (Math|Conversions|ToFloat(Integer) (Math|Conversions|ToInteger(Byte) (.LeftS (Utilities|String|Split (.RightS (Utilities|String|Split _contents "+")) "+")))) (Math|Vector|MakeVector (Math|Conversions|ToFloat(Integer) (.RightS (Utilities|String|Split (.LeftS (Utilities|String|Split (.RightS (Utilities|String|Split (.RightS (Utilities|String|Split _contents "+")) "+")) "Y")) "="))) (Math|Conversions|ToFloat(Integer) (.RightS (Utilities|String|Split (.LeftS (Utilities|String|Split (.RightS (Utilities|String|Split (.RightS (Utilities|String|Split _contents "+")) "+")) "Z")) "=" "IgnoreCase" "FromEnd"))) (Math|Conversions|ToFloat(Integer) (.RightS (Utilities|String|Split (.RightS (Utilities|String|Split (.RightS (Utilities|String|Split _contents "+")) "+")) "=" "IgnoreCase" "FromEnd")))) 1))))
  (for _array_element_2 (Variables|Default|GetNewVar_6)
    (bind (_contents_2 _returnvalue_2) (Class|BuildingSystem|LoadStringfromFile (Utilities|String|Append (Class|KismetSystemLibrary|GetProjectSavedDirectory) "SA" (Utilities|String|ToString(Integer) _array_element_2))))
    (if _returnvalue_2
      (Utilities|Array|Add (Variables|Default|GetNewVar_3) (Utilities|Struct|MakeLightData (Math|Conversions|ToInteger(Byte) (.LeftS (Utilities|String|Split _contents_2 "+"))) (Math|Conversions|ToFloat(Integer) (Math|Conversions|ToInteger(Byte) (.LeftS (Utilities|String|Split (.RightS (Utilities|String|Split _contents_2 "+")) "+")))) (Math|Vector|MakeVector (Math|Conversions|ToFloat(Integer) (.RightS (Utilities|String|Split (.LeftS (Utilities|String|Split (.RightS (Utilities|String|Split (.RightS (Utilities|String|Split _contents_2 "+")) "+")) "Y")) "="))) (Math|Conversions|ToFloat(Integer) (.RightS (Utilities|String|Split (.LeftS (Utilities|String|Split (.RightS (Utilities|String|Split (.RightS (Utilities|String|Split _contents_2 "+")) "+")) "Z")) "=" "IgnoreCase" "FromEnd"))) (Math|Conversions|ToFloat(Integer) (.RightS (Utilities|String|Split (.RightS (Utilities|String|Split (.RightS (Utilities|String|Split _contents_2 "+")) "+")) "=" "IgnoreCase" "FromEnd")))) 2))))
  (bind _returnvalue_3 (SaveGame|CreateSaveGameObject "/Game/Common/ADataSave.ADataSave_C"))
  (Variables|/Game/Common/ADataSave.ADataSave_C|SetAData _returnvalue_3 (Variables|Default|GetNewVar_1))
  (Variables|/Game/Common/ADataSave.ADataSave_C|SetLData _returnvalue_3 (Variables|Default|GetNewVar_3))
  (SaveGame|SaveGametoSlot _returnvalue_3 "14403"))